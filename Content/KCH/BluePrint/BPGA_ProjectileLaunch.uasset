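; Gameplay Ability for enemy ranged attacks that launches a projectile hitbox at the player.
; Plays the owning BP_BaseEnemy's AttackMontage and waits once for a gameplay event, tagged InputUserSettings.Profiles.Default, on the owner.
; The event spawns BP_HitBox_Projectile at the enemy's transform and launches it toward player pawn 0's current location.
; Montage blend-out, interruption or cancellation ends the ability, which prints a debug string on end.
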(event Ability|EventActivateAbility
  (bind _returnvalue (Ability|GetOwningActorfromActorInfo))
  (bind _asbp_base_enemy (Utilities|Casting|CastToBP_BaseEnemy (Ability|GetOwningActorfromActorInfo)))
  (|PlayMontageandWaitProxy "None" (Variables|/Script/LMS_TeamProject.BaseEnemyCharacter|GetAttackMontage _asbp_base_enemy) 1.0 "None" true 1.0 0.0 false
    (:then
      (Ability|Async|WaitGameplayEventToActor _returnvalue "(TagName=\"InputUserSettings.Profiles.Default\")" true
        (:EventReceived
          (bind _returnvalue_2 (Game|SpawnActorfromClass "/Game/KCH/BluePrint/BP_HitBox_Projectile.BP_HitBox_Projectile_C" (Math|Transform|MakeTransform (Transformation|GetActorLocation _returnvalue) (Transformation|GetActorRotation _returnvalue) "1.000000,1.000000,1.000000") "Undefined" "MultiplyWithRoot" _returnvalue 0))
          (Class|HitBoxProjectile|LaunchtoTarget _returnvalue_2 (Transformation|GetActorLocation (Game|Player|GetPlayerPawn 0))))))
    (:OnBlendOut
      (Ability|EndAbility :!label _label))
    (:OnInterrupted
      (goto _label))
    (:OnCancelled
      (goto _label))))

(event Ability|EventOnEndAbility
  (params (bWasCancelled :type Boolean))
  (Development|PrintString "Hello"))