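; Gameplay ability that makes a BP_BaseEnemy fire a projectile hitbox during its attack montage.
; It plays the enemy's AttackMontage and waits for a gameplay event, tagged InputUserSettings.Profiles.Default, on the owner.
; Each event spawns a BP_HitBox_Projectile at the owner's transform and calls LaunchToTarget with a scaled forward vector.
; The ability ends when the montage blends out, is interrupted or is cancelled, with a debug print on end.
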(event Ability|EventActivateAbility
  (bind _returnvalue (Ability|GetOwningActorfromActorInfo))
  (bind _asbp_base_enemy (Utilities|Casting|CastToBP_BaseEnemy (Ability|GetOwningActorfromActorInfo)))
  (|PlayMontageandWaitProxy "None" (Variables|/Script/LMS_TeamProject.BaseEnemyCharacter|GetAttackMontage _asbp_base_enemy) 1.0 "None" true 1.0 0.0 false
    (:then
      (Ability|Async|WaitGameplayEventToActor _returnvalue "(TagName=\"InputUserSettings.Profiles.Default\")"
        (:EventReceived
          (bind _returnvalue_2 (Game|SpawnActorfromClass "/Game/KCH/BluePrint/BP_HitBox_Projectile.BP_HitBox_Projectile_C" (Transformation|GetActorTransform _returnvalue) "Undefined" "MultiplyWithRoot" _returnvalue 0))
          (Class|HitBoxProjectile|LaunchtoTarget _returnvalue_2 (* (Transformation|GetActorForwardVector _returnvalue) 5e+02)))))
    (:OnBlendOut
      (Ability|EndAbility :!label _label))
    (:OnInterrupted
      (goto _label))
    (:OnCancelled
      (goto _label))))

(event Ability|EventOnEndAbility
  (params (bWasCancelled :type Boolean))
  (Development|PrintString "Hello"))